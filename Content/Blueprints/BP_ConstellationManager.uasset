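; Constellation game manager that spawns a fixed first constellation, then a shuffled list one at a time, and times the run.
; Each completion destroys the current constellation, spawns the next and rebinds its completion and interaction events.
; A long timer handle serves as stopwatch, unpaused on first interaction, paused on last, and shown each Tick on BP_Stopwatch's widget.
; When all finish, it shows total duration and raises the stopwatch via timeline.
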(event Custom|StopwatchFunc)

(event Custom|OnFirstInteraction
  (Utilities|Time|UnpauseTimerbyHandle (Variables|Default|GetStopwatch)))

(event Custom|OnConstellationCompleted
  (bind _constellation (Variables|Default|GetConstellation))
  ;[1 1 1] On Constellation Completed
  (CallFunction|HandleConstellationCompleted)
  (Utilities|IsValid _constellation
    (:Is%20Valid
      (EventDispatchers|BindEventtoOnCompleted _constellation (delegate Custom|OnConstellationCompleted))
      (EventDispatchers|BindEventtoOnFirstInteraction _constellation (delegate Custom|OnFirstInteraction))
      (EventDispatchers|BindEventtoOnLastInteraction _constellation (delegate Custom|OnLastInteraction)))))

(event Custom|OnLastInteraction
  (Utilities|Time|PauseTimerbyHandle (Variables|Default|GetStopwatch)))

(event Custom|MoveStopwatch
  (bind _stopwatchbp (Variables|Default|GetStopwatchBP))
  (bind _returnvalue (Transformation|GetActorLocation _stopwatchbp))
  (bind _newtrack_0 (Timeline|Timeline_0 PlayFromStart)
    (:Update
      (Transformation|SetActorLocation _stopwatchbp (Math|Vector|MakeVector (.x _returnvalue) (.y _returnvalue) (Math|Float|Lerp -4.5e+03 -2e+03 _newtrack_0)) false false))))

(event EventBeginPlay
  (Utilities|FlowControl|Sequence
    (:then_0
      (CallFunction|SpawnConstellation)
      (CallFunction|SpawnStopwatch))
    (:then_1
      (Utilities|Array|Shuffle (Variables|Default|GetConstellations))
      (bind _returnvalue (Utilities|Time|SetTimerbyFunctionName 0 "StopwatchFunc" 3.6e+03)) ; Start Stopwatch
      (bind _output_get (Variables|Default|SetStopwatch _returnvalue))
      (Utilities|Time|PauseTimerbyHandle _output_get))
    (:then_2
      (EventDispatchers|BindEventtoOnCompleted (Variables|Default|GetConstellation) (delegate Custom|OnConstellationCompleted)))
    (:then_3
      (EventDispatchers|BindEventtoOnFirstInteraction (Variables|Default|GetConstellation) (delegate Custom|OnFirstInteraction)))
    (:then_4
      (EventDispatchers|BindEventtoOnLastInteraction (Variables|Default|GetConstellation) (delegate Custom|OnLastInteraction)))))

(event EventTick
  (params (DeltaSeconds :type Float%20%28single-precision%29))
  (bind _stopwatch (Variables|Default|GetStopwatch))
  (bind _returnvalue (Class|KismetSystemLibrary|GetTimerElapsedTimeHandle _stopwatch))
  ;[1 1 1] Update stopwatch
  (if (not (Class|KismetSystemLibrary|IsTimerPausedHandle _stopwatch))
    (Rendering|Components|TextRender|SetText (Variables|/Game/Blueprints/Widgets/W_Stopwatch.W_Stopwatch_C|GetTimeText (Variables|Default|GetStopwatchWidget)) (Utilities|Text|FormatText "{sec}:{dec}" (Utilities|Text|ToText(Float) _returnvalue "HalfToEven" false true 2 2 0 0) (Utilities|Text|ToText(Float) (* (Math|Float|%(Float) _returnvalue 1.0) 1e+02) "HalfToEven" false true 2 2 0 0)))))

(fn ConstructionScript)

(fn SpawnNextConstellation
  (bind _returnvalue (Game|SpawnActorfromClass (Utilities|Array|Get(acopy) (Variables|Default|GetConstellations) (Variables|Default|GetConstellationInt)) (Math|Transform|MakeTransform "11535.000000,0.000000,0.000000" "0,174.397202, 0" "1,1,1") "Undefined" 0 0))
  (Variables|Default|SetConstellation _returnvalue))

(fn SpawnConstellation
  (bind _returnvalue (Game|SpawnActorfromClass (Variables|Default|GetFirstConstellation) (Math|Transform|MakeTransform "11535.000000,0.000000,-0.000000" "0,174.397202, 0" "1,1,1") "Undefined" 0 0))
  (Variables|Default|SetConstellation _returnvalue))

(fn SpawnStopwatch
  (bind _returnvalue (Game|SpawnActorfromClass "/Game/Blueprints/BP_Stopwatch.BP_Stopwatch_C" (Math|Transform|MakeTransform "11300.000000, 0,-4500.000000" "0,180.000000, 0" "20.000000,20.000000,20.000000") "Undefined" 0 0))
  (bind _output_get (Variables|Default|SetStopwatchBP _returnvalue))
  (bind _asw_stopwatch (Utilities|Casting|CastToW_Stopwatch (UserInterface|GetWidget (Variables|/Game/Blueprints/BP_Stopwatch.BP_Stopwatch_C|GetWidget _output_get))))
  (Variables|Default|SetStopwatchWidget _asw_stopwatch))

(fn HandleGameEnd
  (bind _stopwatch (Variables|Default|GetStopwatch))
  (bind _returnvalue (Class|KismetSystemLibrary|GetTimerElapsedTimeHandle _stopwatch))
  (bind _returnvalue_2 (Utilities|Text|ToText(Float) _returnvalue "HalfToEven" false true 2 2 0 0))
  (bind _returnvalue_3 (Math|Float|%(Float) _returnvalue 1.0))
  (bind _returnvalue_4 (* _returnvalue_3 1e+02))
  (bind _returnvalue_5 (Utilities|Text|ToText(Float) _returnvalue_4 "HalfToEven" false true 2 2 0 0))
  (bind _result (Utilities|Text|FormatText "{sec}:{dec}" _returnvalue_2 _returnvalue_5))
  (bind _result_2 (Utilities|Text|FormatText "Total duration: {Time}" _result))
  (Development|PrintText "All constellations are done")
  (Utilities|Time|PauseTimerbyHandle _stopwatch)
  (Development|PrintText _result_2 true true "(R=0.017264,G=1.000000,B=0.382847,A=1.000000)" 1e+01)
  (Rendering|Components|TextRender|SetText (Variables|/Game/Blueprints/Widgets/W_Stopwatch.W_Stopwatch_C|GetTimeText (Variables|Default|GetStopwatchWidget)) _result_2)
  (CallFunction|MoveStopwatch))

(fn HandleConstellationCompleted
  (Actor|DestroyActor (Variables|Default|GetConstellation))
  (if (< (Variables|Default|GetConstellationInt) (Utilities|Array|Length (Variables|Default|GetConstellations)))
    (CallFunction|SpawnNextConstellation)
    (Math|Integer|IncrementInt (Variables|Default|GetConstellationInt))
    (else
      (CallFunction|HandleGameEnd) ; All constellations completed
    )))