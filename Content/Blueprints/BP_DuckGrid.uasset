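; BP_DuckGrid runs a VR duck-shooting minigame, spawning ducks at hidden points built in the construction script.
; A looping timer picks random points, avoiding immediate repeats, and passes speed and grid reference to each duck.
; Hits update the score sign, while ducks crossing the barrier cost bells until MiniGameCube ends the game.
; A difficulty timer raises duck speed and shrinks SpawnInterval, though the running spawn timer is never reset.
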(event OnComponentBeginOverlap(Barrier)
  (params (OverlappedComponent :type Primitive%20Component%20Object%20Reference) (OtherActor :type Actor%20Object%20Reference) (OtherComp :type Primitive%20Component%20Object%20Reference) (OtherBodyIndex :type Integer) (bFromSweep :type Boolean) (SweepResult :type Hit%20Result%20Structure%20%28by%20ref%29))
  ;[1 1 1] Keep track of stolen bells (ducks that crossed barrier)
  (bind _asbp_duck_2 (Utilities|Casting|CastToBP_Duck2 OtherActor))
  (bind _result (Math|Integer|DecrementInt (Variables|Default|GetAmountOfBells))
    (:%20%20
      (Actor|DestroyActor _asbp_duck_2) ; Duck diving animation before this node
      (if (<= (Variables|Default|GetAmountOfBells) 0)
        (Default|OnGameOver (Variables|Default|GetMiniGameCube))))))

(event Custom|SpawnDuckEvent
  ;[1 1 1] Spawn Duck
  (bind _int (CallFunction|GetSpawnInt))
  (Variables|Default|SetPrevSpawnInt _int)
  (CallFunction|SpawnDuck (Transformation|GetWorldTransform (Utilities|Array|Get(acopy) (Variables|Default|GetDuckSpawnPoints) _int))))

(event Custom|OnDuckHit
  ;[1 1 1] Update score when projectile hit duck
  (bind _result (Math|Integer|IncrementInt (Variables|Default|GetScore))
    (:%20%20
      (bind _asbp_duck_score_sign (Utilities|Casting|CastToBP_DuckScoreSign (Variables|/Script/Engine.ChildActorComponent|GetChildActor (Variables|Default|GetScoreSign))))
      (bind _asw_duck_score (Utilities|Casting|CastToW_DuckScore (UserInterface|GetWidget (Variables|/Game/Blueprints/BP_DuckScoreSign.BP_DuckScoreSign_C|GetScore _asbp_duck_score_sign))))
      (Default|SetScore _asw_duck_score _result))))

(event EventBeginPlay
  (Utilities|FlowControl|Sequence
    (:then_0
      (Utilities|Time|SetTimerbyFunctionName self "IncreaseDifficulty" (Variables|Default|GetIncreaseDifficultyInterval) true))
    (:then_1
      (Utilities|Time|SetTimerbyEvent (delegate Custom|SpawnDuckEvent) (Variables|Default|GetSpawnInterval) true)
      (Utilities|Array|Clear (Variables|Default|GetDucks))
      (bind _rotation (CallFunction|FindLookatPlayerRotation (Variables|Default|GetWidget)))
      (Transformation|SetWorldRotation (Variables|Default|GetWidget) _rotation false false))))

(fn ConstructionScript
  (Utilities|Array|Clear (Variables|Default|GetDuckSpawnPoints))
  ;[1 1 1] Spawn spawn points
  (for _index (range 0 (- (Variables|Default|GetAmountOfSpawnPoints) 1))
    (bind _returnvalue (AddComponent|AddStaticMeshComponent false (Math|Transform|MakeTransform (Utilities|CalculateLocation _index) "0, 0, 0" "0.100000,0.100000,0.100000")))
    (Utilities|Array|Add (Variables|Default|GetDuckSpawnPoints) _returnvalue)
    (Components|StaticMesh|SetStaticMesh _returnvalue "/Engine/EditorMeshes/EditorSphere.EditorSphere")
    (Rendering|Material|SetMaterial _returnvalue 0 "/Engine/VREditor/UI/FrameMaterial.FrameMaterial")
    (Collision|SetCollisionEnabled _returnvalue "QueryOnly")
    (Development|SetHiddeninGame _returnvalue true false)))

(fn SpawnDuck
  (params (Transform :type Transform))
  (bind _returnvalue (Game|SpawnActorfromClass "/Game/Blueprints/BP_Duck2.BP_Duck2_C" (Math|Transform|MakeTransform (.location Transform) "0,180.000000, 0" "0.100000,0.100000,0.100000") "Undefined" 0 0))
  (Utilities|Array|Add (Variables|Default|GetDucks) _returnvalue)
  (Variables|/Game/Blueprints/BP_Duck2.BP_Duck2_C|SetMoveSpeed _returnvalue (Variables|Default|GetDuckMoveSpeed))
  (Variables|/Game/Blueprints/BP_Duck2.BP_Duck2_C|SetDuckGridRef _returnvalue self))

(fn SetMiniGameCube
  (params (MiniGameCube :type BP%20I%20Duck%20Game%20Object%20Reference))
  (Variables|Default|SetMiniGameCube MiniGameCube))

(fn DestroyAllDucks
  (bind _arrayelement (Utilities|Array|ReverseforEachLoop (Variables|Default|GetDucks))
    (:LoopBody
      (Actor|DestroyActor _arrayelement))))

(fn FindLookatPlayerRotation
  (params (Widget :type Widget%20Component%20Object%20Reference))
  (bind _asbp_vrpawn (Utilities|Casting|CastToBP_VRPawn (Game|Player|GetPlayerPawn 0)))
  (return (Math|Rotator|FindLookatRotation (Transformation|GetWorldLocation Widget) (Transformation|GetWorldLocation (Variables|/PicoMobile/BP_Pico_Pawn.BP_Pico_Pawn_C|GetCamera _asbp_vrpawn)))))

(fn IncreaseDifficulty
  (Utilities|FlowControl|Sequence
    (:then_0
      (Variables|Default|SetDuckMoveSpeed (* (Variables|Default|GetDuckMoveSpeed) 1.2)))
    (:then_1
      (Variables|Default|SetSpawnInterval (* (Variables|Default|GetSpawnInterval) 0.2)))))

(fn GetSpawnInt
  (bind _amountofspawnpoints (Variables|Default|GetAmountOfSpawnPoints))
  (bind _returnvalue (- _amountofspawnpoints 1))
  (Variables|Default|SetRandomInt (Math|Random|RandomIntegerinRange 0 _returnvalue))
  (if (!= (Variables|Default|GetPrevSpawnInt) (Variables|Default|GetRandomInt))
    (return (Variables|Default|GetRandomInt))
    (elif (== (Variables|Default|GetRandomInt) _returnvalue)
      (return (+ (Variables|Default|GetRandomInt) -1))
      (else
        (return (+ (Variables|Default|GetRandomInt) 1))))))