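; BP_I_Star is an interactable star that serves as a selectable point within a constellation.
; On BeginPlay it caches its parent actor as a BP_ConstellationBase, printing a message if the cast fails.
; It is always interactable and passes itself to the constellation's OnStarInteraction, which handles the interaction.
; SetIndicatorVisibility shows or hides the indicator inside its W_Star widget.
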(event EventBeginPlay
  (bind _asbp_constellation_base (Utilities|Casting|CastToBP_ConstellationBase (Actor|GetParentActor))
    (:then
      (Variables|Default|SetConstellation _asbp_constellation_base))
    (:CastFailed
      (Development|PrintText "Cast to BP_Constellation failed"))))

(event EventInteract
  ;[1 1 1] Try to attach line to pointer
  (Default|OnStarInteraction (Variables|Default|GetConstellation) self))

(fn ConstructionScript)

(fn SetIndicatorVisibility
  (params (IsVisible :type Boolean))
  (bind _asw_star (Utilities|Casting|CastToW_Star (UserInterface|GetWidget (Variables|Default|GetWidget))))
  (if IsVisible
    (Widget|SetVisibility (Variables|/Game/Blueprints/Widgets/W_Star.W_Star_C|GetIndicator _asw_star) "Visible")
    (else
      (Widget|SetVisibility (Variables|/Game/Blueprints/Widgets/W_Star.W_Star_C|GetIndicator _asw_star) "Hidden"))))

(fn IsInteractable
  (return true))