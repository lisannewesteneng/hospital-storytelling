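; Interactable item that takes the player out of the telescope's constellation view.
; On Interact it teleports the player pawn back to its original location, makes the sky sphere mesh visible again and unloads the streamed Constellations level without blocking.
; It always reports as interactable and supplies a fixed timer length.
; An unconnected branch that toggles between the Main and Constellations maps with Open Level never runs.
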(event EventInteract
  (Transformation|SetActorLocation (Game|Player|GetPlayerPawn 0) (Variables|Default|GetOriginal%20Player%20Location) false true)
  (Rendering|SetVisibility (Variables|/Engine/EngineSky/BP_Sky_Sphere.BP_Sky_Sphere_C|GetSkySphereMesh (Utilities|ResolveSoftReference (Variables|Default|GetSkySphere))) true false)
  (Class|GameplayStatics|UnloadStreamLevelbySoftObjectPtr "/Game/Maps/Constellations.Constellations" false))

(fn ConstructionScript)

(fn GetTimerLength
  (return 3.0))

(fn IsInteractable
  (return true))