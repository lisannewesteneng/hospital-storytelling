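; Interactable test cube that cycles the visibility of two referenced water meshes.
; On BeginPlay only Water1 shows, then successive interactions show only Water2, hide both, and return to Water1.
; A switch picks the state, and an integer counter increments after each interaction, resetting at the last state to loop.
; It is always interactable with a zero timer length, and leftover Water3 visibility calls never run.
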(event EventBeginPlay
  (Rendering|SetVisibility (Variables|/Script/Engine.StaticMeshActor|GetStaticMeshComponent (Variables|Default|GetWater1)) true false)
  (Rendering|SetVisibility (Variables|/Script/Engine.StaticMeshActor|GetStaticMeshComponent (Variables|Default|GetWater2)) false false))

(event EventInteract
  (Utilities|FlowControl|Sequence
    (:then_0
      (switch int (stale _result)
        (:0
          (Rendering|SetVisibility (Variables|/Script/Engine.StaticMeshActor|GetStaticMeshComponent (Variables|Default|GetWater1)) false false)
          (Rendering|SetVisibility (Variables|/Script/Engine.StaticMeshActor|GetStaticMeshComponent (Variables|Default|GetWater2)) true false))
        (:1
          (Rendering|SetVisibility (Variables|/Script/Engine.StaticMeshActor|GetStaticMeshComponent (Variables|Default|GetWater1)) false false)
          (Rendering|SetVisibility (Variables|/Script/Engine.StaticMeshActor|GetStaticMeshComponent (Variables|Default|GetWater2)) false false))
        (:2
          (Rendering|SetVisibility (Variables|/Script/Engine.StaticMeshActor|GetStaticMeshComponent (Variables|Default|GetWater1)) true false)
          (Rendering|SetVisibility (Variables|/Script/Engine.StaticMeshActor|GetStaticMeshComponent (Variables|Default|GetWater2)) false false)
          (Variables|Default|Setint -1))))
    (:then_1
      (bind _result (Math|Integer|IncrementInt (Variables|Default|Getint))))))

(fn ConstructionScript)

(fn GetTimerLength
  (return 0.0))

(fn IsInteractable
  (return true))