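; Interactable object that starts and stops a VR duck shooting mini-game.
; Interact toggles the pawn's shooter mode, spawning a BP_DuckGrid that a timeline raises into view, or clearing its ducks, lowering and destroying it.
; The grid receives a reference to this actor.
; OnGameOver stops the shooter, shows the game-over sign, then runs the same teardown after a delay, with interaction blocked meanwhile.
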(event Custom|OnGameOver
  (bind _duckgrid (Variables|Default|GetDuckGrid))
  (bind _spawnlocation (Variables|Default|GetSpawnLocation))
  (bind (_x _y) (Math|Vector|BreakVector _spawnlocation))
  ;[1 1 1] On Game Over
  (Variables|Default|SetIsGameOver true)
  (Default|StopShooter (stale EventInteract _asbp_vrpawn))
  (Default|ShowGameOverSign (Variables|Default|GetDuckGrid))
  (Utilities|FlowControl|Delay (Variables|Default|GetGameOverTextDuration))
  ;[1 1 1] Stop shooting game
  (Default|StopShooter (stale EventInteract _asbp_vrpawn))
  (Default|DestroyAllDucks _duckgrid)
  (bind _newtrack_0 (Timeline|Timeline_1 ReverseFromEnd)
    (:Update
      (Transformation|SetActorLocation _duckgrid (Math|Vector|MakeVector _x _y (Math|Float|Lerp -61.0 6.0 _newtrack_0)) false false))
    (:Finished
      (Actor|DestroyActor _duckgrid)
      (Variables|Default|SetIsShooting false)
      (Variables|Default|SetIsGameOver false))))

(event EventInteract
  (bind _duckgrid (Variables|Default|GetDuckGrid))
  (bind _spawnlocation (Variables|Default|GetSpawnLocation))
  (bind _spawnlocation_2 (Variables|Default|GetSpawnLocation))
  (bind (_x _y) (Math|Vector|BreakVector _spawnlocation_2))
  (bind (_x_2 _y_2) (Math|Vector|BreakVector _spawnlocation))
  (bind _asbp_vrpawn (Utilities|Casting|CastToBP_VRPawn (Game|Player|GetPlayerPawn 0)))
  (if (not (Variables|Default|GetIsGameOver))
    (if (Variables|Default|GetIsShooting)
      ;[1 1 1] Stop shooting game
      (Default|StopShooter _asbp_vrpawn)
      (Default|DestroyAllDucks _duckgrid)
      (bind _newtrack_0 (Timeline|Timeline_1 ReverseFromEnd)
        (:Update
          (Transformation|SetActorLocation _duckgrid (Math|Vector|MakeVector _x_2 _y_2 (Math|Float|Lerp -61.0 6.0 _newtrack_0)) false false))
        (:Finished
          (Actor|DestroyActor _duckgrid)
          (Variables|Default|SetIsShooting false)
          (Variables|Default|SetIsGameOver false)))
      (else
        ;[1 1 1] Start shooting game
        (Default|StartShooter _asbp_vrpawn)
        (bind _spawnedgrid (CallFunction|InitGrid))
        (bind _newtrack_0_2 (Timeline|Timeline_0 PlayFromStart)
          (:Update
            (Transformation|SetActorLocation _spawnedgrid (Math|Vector|MakeVector _x _y (Math|Float|Lerp -61.0 6.0 _newtrack_0_2)) false false))
          (:Finished
            (Rendering|SetVisibility (Variables|/Game/Blueprints/BP_DuckGrid.BP_DuckGrid_C|GetScoreSign _spawnedgrid) true false)
            (Variables|Default|SetIsShooting true)))))))

(fn ConstructionScript)

(fn InitGrid
  (bind _returnvalue (Game|SpawnActorfromClass "/Game/Blueprints/BP_DuckGrid.BP_DuckGrid_C" (Math|Transform|MakeTransform (Variables|Default|GetSpawnLocation) "0,-90.000000, 0" "1,1,1") "Undefined" 0 0))
  (bind _output_get (Variables|Default|SetDuckGrid _returnvalue))
  (Default|SetMiniGameCube _output_get self)
  (return _returnvalue))

(fn IsInteractable
  (return true))