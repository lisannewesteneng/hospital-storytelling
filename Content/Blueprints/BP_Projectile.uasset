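; BP_Projectile is a short-lived projectile that knocks out BP_Duck2 targets and removes itself two seconds after spawning.
; When its Sphere hits a duck, it calls the duck's OnHit, destroys that duck and turns off bouncing on its ProjectileMovement.
; The first bounce sets the projectile's gravity scale through a DoOnce.
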(event OnComponentHit(Sphere)
  (params (HitComponent :type Primitive%20Component%20Object%20Reference) (OtherActor :type Actor%20Object%20Reference) (OtherComp :type Primitive%20Component%20Object%20Reference) (NormalImpulse :type Vector :default "0, 0, 0") (Hit :type Hit%20Result%20Structure%20%28by%20ref%29))
  (bind _asbp_duck_2 (Utilities|Casting|CastToBP_Duck2 OtherActor))
  (Default|OnHit _asbp_duck_2)
  (Actor|DestroyActor _asbp_duck_2)
  (Variables|/Script/Engine.ProjectileMovementComponent|SetbShouldBounce (Variables|Default|GetProjectileMovement) false))

(event OnProjectileBounce(ProjectileMovement)
  (params (ImpactResult :type Hit%20Result%20Structure%20%28by%20ref%29) (ImpactVelocity :type Vector%20%28by%20ref%29 :default "0, 0, 0"))
  (Utilities|FlowControl|DoOnce false
    (:Completed
      (Variables|/Script/Engine.ProjectileMovementComponent|SetProjectileGravityScale (Variables|Default|GetProjectileMovement) 0.8))))

(event EventBeginPlay
  (Utilities|FlowControl|Delay 2.0)
  (Actor|DestroyActor))

(fn ConstructionScript)