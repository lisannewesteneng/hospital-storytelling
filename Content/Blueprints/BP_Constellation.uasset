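; VR connect-the-stars constellation puzzle where the player draws lines between stars in a set order.
; BeginPlay gathers BP_Star child actors under Plane, repeats one as the ending, and uses widget collision to enable only the next star.
; Each interaction spawns a spline and spline mesh whose free end follows the BP_VRPawn pointer every Tick.
; Overstretching destroys the active line and steps back one star; completing the figure prints "Done!".
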(event Custom|OnStarInteraction
  (params (Star :type Actor%20Object%20Reference))
  ;[1 1 1] Create line, disable star, enable next star
  (CallFunction|CreateLinefromStar Star)
  (CallFunction|EnableStar false (Variables|Default|GetStarInt))
  (bind _result (Math|Integer|IncrementInt (Variables|Default|GetStarInt))
    (:%20%20
      (if (<= _result (- (Utilities|Array|Length (Variables|Default|GetStars)) 1))
        (CallFunction|EnableStar true _result)
        (else
          ;[1 1 1] Figure is done, disable last star and set spline end location
          (CallFunction|EnableStar false (Variables|Default|GetStarInt))
          (Variables|Default|SetCurrentSpline 0)
          (Development|PrintText "Done!"))))))

(event EventTick
  (params (DeltaSeconds :type Float%20%28single-precision%29))
  (CallFunction|UpdateSplinetoPointerPosition)
  (CallFunction|UpdateSplineMesh)
  (CallFunction|CheckSplineLength))

(event EventBeginPlay
  (bind _plane (Variables|Default|GetPlane))
  (bind _children (Components|GetChildrenComponents _plane false))
  ;[1 1 1] Create array of stars
  (Utilities|Array|Clear (Variables|Default|GetStars))
  (for _array_element _children
    (CallFunction|AddtoStarArray _array_element))
  ;[1 1 1] Add ending to array again at the end, enable first star
  (CallFunction|AddtoStarArray (Utilities|Array|Get(acopy) _children 3))
  (CallFunction|EnableStar true))

(fn ConstructionScript)

(fn UpdateSplinetoPointerPosition
  (bind _currentspline (Variables|Default|GetCurrentSpline)
    (:then
      (bind _asbp_vrpawn (Utilities|Casting|CastToBP_VRPawn (Game|Player|GetPlayerPawn 0))
        (:then
          (Spline|SetLocationatSplinePoint _currentspline 1 (Transformation|GetWorldLocation (Variables|/Game/Blueprints/BP_VRPawn.BP_VRPawn_C|GetPointerWidget _asbp_vrpawn)) "World" true))
        (:CastFailed
          (Development|PrintText "Cast to BP_VRPawn failed"))))
    (:else)))

(fn UpdateSplineMesh
  (bind _currentspline (Variables|Default|GetCurrentSpline)
    (:then
      (bind _splinemesh (Variables|Default|GetSplineMesh)
        (:then
          (SplineMesh|SetStartandEnd _splinemesh (.Location (Spline|GetLocationandTangentatSplinePoint _currentspline 0 "Local")) (.Tangent (Spline|GetLocationandTangentatSplinePoint _currentspline 0 "Local")) (.Location (Spline|GetLocationandTangentatSplinePoint _currentspline 1 "Local")) (.Tangent (Spline|GetLocationandTangentatSplinePoint _currentspline 1 "Local")) true :!class /Script/Engine.SplineMeshComponent))
        (:else)))
    (:else)))

(fn CreateLinefromStar
  (params (Star :type Actor%20Object%20Reference))
  (bind _returnvalue (AddComponent|AddSplineComponent false))
  (Utilities|FlowControl|Sequence
    (:then_0
      (Spline|SetSplinePointType _returnvalue 0 "Curve" true) ; To Do: Can this node be deleted?
      (Spline|SetLocationatSplinePoint _returnvalue 0 (Transformation|GetActorLocation Star) "World" true))
    (:then_1
      (Spline|SetSplinePointType _returnvalue 1 "Curve" true) ; To Do: Can this node be deleted?
      (Variables|Default|SetCurrentSpline _returnvalue))
    (:then_2
      (bind _returnvalue_2 (AddComponent|AddSplineMeshComponent false))
      (Variables|Default|SetSplineMesh _returnvalue_2))))

(fn EnableStar
  (params (Enable :type Boolean) (Index :type Integer))
  (bind _stars (Variables|Default|GetStars))
  (bind _output (Utilities|Array|Get(acopy) _stars Index))
  (bind _widget (Variables|/Game/Blueprints/BP_Star.BP_Star_C|GetWidget _output))
  (Utilities|IsValid _output
    (:Is%20Valid
      (if Enable
        (Collision|SetCollisionEnabled _widget "QueryOnly") ; Enable Collision
        (else
          (Collision|SetCollisionEnabled _widget "NoCollision") ; Disable Collision
        )))))

(fn CheckSplineLength
  (bind _currentspline (Variables|Default|GetCurrentSpline)
    (:then
      (if (> (Spline|GetSplineLength _currentspline) (Variables|Default|GetMaxSplineLength))
        (Utilities|FlowControl|Sequence
          (:then_0
            (Components|DestroyComponent (Variables|Default|GetCurrentSpline))
            (Components|DestroyComponent (Variables|Default|GetSplineMesh)))
          (:then_1
            (CallFunction|EnableStar false (Variables|Default|GetStarInt))
            (bind _result (Math|Integer|DecrementInt (Variables|Default|GetStarInt))
              (:%20%20
                (CallFunction|EnableStar true _result)))))))
    (:else)))

(fn AddtoStarArray
  (params (StarComponent :type Scene%20Component%20Object%20Reference))
  (bind _aschild_actor_component (Utilities|Casting|CastToChildActorComponent StarComponent))
  (bind _asbp_star (Utilities|Casting|CastToBP_Star (Variables|/Script/Engine.ChildActorComponent|GetChildActor _aschild_actor_component)))
  (Utilities|Array|Add (Variables|Default|GetStars) _asbp_star)
  (Collision|SetCollisionEnabled (Variables|/Game/Blueprints/BP_Star.BP_Star_C|GetWidget _asbp_star) "NoCollision"))