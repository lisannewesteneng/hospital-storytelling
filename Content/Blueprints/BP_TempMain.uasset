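; Temporary main Blueprint that drives a day/night cycle by rotating a light source and refreshing the sky sphere's sun direction.
; TimeCycle starts on BeginPlay and loops itself through a short Delay instead of Tick, scaling rotation by frame delta and day length.
; A narrow pitch window below zero triggers a resettable DoOnce into a FlipFlop, alternating StartDay, which increments and prints the day counter, with StartNight, which only prints.
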(event Custom|TimeCycle
  (bind _returnvalue (Transformation|GetActorRotation "Literal"))
  (Transformation|AddActorLocalRotation "Literal" (Math|Rotator|MakeRotator 0.0 (* (Utilities|Time|GetWorldDeltaSeconds) (/ 5e+02 (Variables|Default|GetDay%20Length%20in%20Seconds))) 0.0) false false) ; target is light source
  (Default|UpdateSunDirection "Literal") ; target is skysphere
  (if (and (< (.pitch _returnvalue) 0.0) (> (.pitch _returnvalue) -5.0))
    (Utilities|FlowControl|Sequence
      (:then_0
        (Utilities|FlowControl|DoOnce false :!label _label
          (:Completed
            (Utilities|FlowControl|FlipFlop
              (:A
                (CallFunction|StartDay))
              (:B
                (CallFunction|StartNight))))))
      (:then_1
        (Utilities|FlowControl|Delay 0.01 :!label _label_2)
        (CallFunction|TimeCycle)))
    (else
      (Utilities|FlowControl|Sequence
        (:then_0
          (goto _label Reset))
        (:then_1
          (goto _label_2))))))

(event Custom|StartDay
  (bind _result (Math|Integer|IncrementInt (Variables|Default|GetDay%20Counter))
    (:%20%20
      (Development|PrintString (Utilities|String|Append "Start day " (Utilities|String|ToString(Integer) _result))))))

(event Custom|StartNight
  (Development|PrintText "Start Night"))

(event EventBeginPlay
  (CallFunction|TimeCycle))

(event EventTick
  (params (DeltaSeconds :type Float%20%28single-precision%29)))

(fn ConstructionScript)