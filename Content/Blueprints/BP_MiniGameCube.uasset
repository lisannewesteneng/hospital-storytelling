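; BP_MiniGameCube is an interactable cube that toggles a VR duck-shooting minigame on and off through a FlipFlop.
; Starting enables the pawn's shooter, spawns a BP_DuckGrid linked to the cube, and teleports the player, saving their location.
; Stopping disables shooting, destroys the grid and ducks, and returns the player.
; Game over stops shooting, shows the grid's widget, then after a delay re-enters the same FlipFlop.
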(event Custom|OnGameOver
  (bind _duckgrid (Variables|Default|GetDuckGrid))
  ;[1 1 1] On Game Over
  (Default|StopShooter (stale EventInteract _asbp_vrpawn))
  (Rendering|SetVisibility (Variables|/Game/Blueprints/BP_DuckGrid.BP_DuckGrid_C|GetWidget (Variables|Default|GetDuckGrid)) true false)
  (Utilities|FlowControl|Delay (Variables|Default|GetGameOverTextDuration))
  (Utilities|FlowControl|FlipFlop
    (:A
      ;[1 1 1] Start shooting game
      (Default|StartShooter (stale EventInteract _asbp_vrpawn))
      (CallFunction|InitGrid)
      (Variables|Default|SetOriginalPlayerLocation (Transformation|GetActorLocation (stale EventInteract _asbp_vrpawn)))
      (Transformation|Teleport (stale EventInteract _asbp_vrpawn) (Variables|Default|GetPlayerLocation) "0,90.000000, 0"))
    (:B
      ;[1 1 1] Stop shooting game
      (Default|StopShooter (stale EventInteract _asbp_vrpawn))
      (Default|DestroyAllDucks _duckgrid)
      (Actor|DestroyActor _duckgrid)
      (Transformation|Teleport (stale EventInteract _asbp_vrpawn) (Variables|Default|GetOriginalPlayerLocation) "0, 0, 0"))))

(event EventInteract
  (bind _duckgrid (Variables|Default|GetDuckGrid))
  (bind _asbp_vrpawn (Utilities|Casting|CastToBP_VRPawn (Game|Player|GetPlayerPawn 0)))
  (Utilities|FlowControl|FlipFlop
    (:A
      ;[1 1 1] Start shooting game
      (Default|StartShooter _asbp_vrpawn)
      (CallFunction|InitGrid)
      (Variables|Default|SetOriginalPlayerLocation (Transformation|GetActorLocation _asbp_vrpawn))
      (Transformation|Teleport _asbp_vrpawn (Variables|Default|GetPlayerLocation) "0,90.000000, 0"))
    (:B
      ;[1 1 1] Stop shooting game
      (Default|StopShooter _asbp_vrpawn)
      (Default|DestroyAllDucks _duckgrid)
      (Actor|DestroyActor _duckgrid)
      (Transformation|Teleport _asbp_vrpawn (Variables|Default|GetOriginalPlayerLocation) "0, 0, 0"))))

(fn ConstructionScript)

(fn InitGrid
  (bind _returnvalue (Game|SpawnActorfromClass "/Game/Blueprints/BP_DuckGrid.BP_DuckGrid_C" (Math|Transform|MakeTransform (Variables|Default|GetSpawnLocation) "0, 0, 0" "1,1,1") "Undefined" 0 0))
  (bind _output_get (Variables|Default|SetDuckGrid _returnvalue))
  (Default|SetMiniGameCube _output_get self)
  (Rendering|SetVisibility (Variables|/Game/Blueprints/BP_DuckGrid.BP_DuckGrid_C|GetWidget _output_get) false false))

(fn IsInteractable
  (return true))